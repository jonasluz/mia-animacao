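; Spawner actor that creates a bouncing ball at its Arrow on BeginPlay, either physics-driven or animated.
; SpawnBola destroys any previous animated ball, spawns BolaBlueprint, then either launches it with VerticalImpulse or stores it and calls Animate, based on UsePhysics.
; Tick polls the animated ball and, once it is Finished, opens MainMap after a short Delay.
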(event `self.ReceiveBeginPlay`
  (`self.Spawn_Bola`))

(event `self.ReceiveTick`
  (params (DeltaSeconds :type "Float (single-precision)"))
  (bind _animatingbola (`self.AnimatingBola`))
  (`/Engine/EditorBlueprintResources/StandardMacros.IsValid` _animatingbola
    (:`Is Valid`
      (if (`/Game/Blueprints/BolaQueQuica_BP.Finished` _animatingbola)
        (`KismetSystemLibrary.Delay` 0.2)
        (`GameplayStatics.OpenLevel` "MainMap")))))

(fn `Spawn_Bola`
  (bind _animatingbola (`self.AnimatingBola`))
  ;[1 1 1] Cria nova bola
  (`/Engine/EditorBlueprintResources/StandardMacros.IsValid` _animatingbola
    (:`Is Valid`
      (`self.K2_DestroyActor` _animatingbola))
    (:`Is Not Valid`
      _))
  (bind _returnvalue (`|SpawnActorFromClass` (`self.Bola_Blueprint`) (`SceneComponent.K2_GetComponentToWorld` (`self.Arrow`)) "Undefined" "OverrideRootScale"))
  ;[1 1 1] Configura bola
  (bind _asbola_que_quica_bp (cast `/Game/Blueprints/BolaQueQuica_BP` _returnvalue))
  (if (`self.UsePhysics`)
    (set `/Game/Blueprints/BolaQueQuica_BP.VerticalImpulse` (`self.VerticalImpulse`) _asbola_que_quica_bp)
    ;[1 1 1] Ativa bola
    (`/Game/Blueprints/BolaQueQuica_BP.Launch` _asbola_que_quica_bp)
    (else
      (bind _output_get (set `self.AnimatingBola` _asbola_que_quica_bp))
      (`/Game/Blueprints/BolaQueQuica_BP.Animate` _output_get))))

(fn `UserConstructionScript`)