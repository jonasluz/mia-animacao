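; Bouncing ball actor that either fakes its bounce in code or runs on physics, switched by the Animate and Launch functions.
; While physics is off, Tick advances the sphere along Y at a speed proportional to a reference height that decays with distance.
; Actor height follows an absolute sine of travelled distance until it settles at the radius, and the sphere rolls to match.
; Launch enables physics and applies a sideways force along Y.
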(event EventBeginPlay
  ;[1 1 1] Guarda altura inicial
  (bind _output_get (Variables|Animation|SetInitialHeight (.Z (Math|Vector|BreakVector (Transformation|GetActorLocation)))))
  (Variables|Animation|SetDistance _output_get)
  (Variables|Animation|SetFinished false))

(event Collision|EventActorBeginOverlap
  (params (OtherActor :type Actor%20Object%20Reference)))

(event EventTick
  (params (DeltaSeconds :type Float%20%28single-precision%29))
  (CallFunction|AnimationTick DeltaSeconds))

(fn ConstructionScript)

(fn Launch
  (bind _sphere (Variables|Default|GetSphere))
  ;[1 1 1] Configuração
  (Physics|SetSimulatePhysics _sphere true)
  (Physics|AddForce _sphere (Math|Vector|MakeVector 0.0 (* (Variables|Physics|GetVerticalImpulse) 1e+06) 0.0) "None" false) ; Falling from gravity
)

(fn Animate
  (Physics|SetSimulatePhysics (Variables|Default|GetSphere) false) ; Settings
)

(fn AnimationTick
  (params (Delta%20Seconds :type Float%20%28single-precision%29))
  (bind _returnvalue (Transformation|GetActorLocation))
  (bind _sphere (Variables|Default|GetSphere))
  (bind (_x _y) (Math|Vector|BreakVector _returnvalue))
  ;[1 1 1] Precondição: não usar física
  (if (not (Physics|IsSimulatingPhysics (Variables|Default|GetSphere) "None")) ; Se usando física, não anima
    ;[1 1 1] Atualiza Posição
    (bind (_distance_offset _height _rotationinx) (CallFunction|CalculateTransformation Delta%20Seconds)) ; Calcula as posições e atualiza altura de referência
    (Transformation|SetActorLocation (Math|Vector|MakeVector _x _y _height) false false)
    (Transformation|AddWorldOffset _sphere (Math|Vector|MakeVector 0.0 _distance_offset 0.0) false false)
    (Variables|Animation|SetFinished (Math|Float|NearlyEqual(Float) _distance_offset 0.0 0.01))
    (Transformation|AddWorldRotation _sphere (Math|Rotator|MakeRotator _rotationinx 0.0 0.0) false false)))

(fn CalculateTransformation
  (params (Delta%20Seconds :type Float%20%28single-precision%29))
  (bind (_ray _halfcirc) (Utilities|SphereDimensions))
  (bind (_updateddistance _deltadistance) (Utilities|UpdatedDistance Delta%20Seconds))
  ;[1 1 1] Adiciona trecho à distância percorrida
  (bind _output_get (Variables|Animation|SetDistance _updateddistance))
  ;[1 1 1] Dissipa altura de referência
  (bind _output_get_2 (Variables|Animation|SetInitialHeight (Utilities|DissipatedHeight _deltadistance)))
  (if (Math|Float|NearlyEqual(Float) _output_get_2 0.0 _ray)
    (LocalVariables|SetResult _ray)
    (else
      (LocalVariables|SetResult (Utilities|SenoidHeight _output_get))))
  (return _deltadistance (LocalVariables|GetResult) (Utilities|DeltaRotation _deltadistance _halfcirc)))